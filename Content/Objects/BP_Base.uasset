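; BP_Base is a base actor that periodically spawns a wave of creeps.
; Tick drives a countdown, set on BeginPlay, using a one-second Delay to throttle each decrement.
; When the timer runs out, it spawns one melee and one distance creep at the Box component's location, resets the countdown and prints a debug message.
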(event EventBeginPlay
  (bind _output_get (Variables|Default|SetCooldownMaxValue 10))
  (Variables|Default|SetCooldownTimer _output_get))

(event EventTick
  (params (DeltaSeconds :type Float%20%28single-precision%29))
  (bind _box (Variables|Default|GetBox))
  (bind _returnvalue (Transformation|GetWorldLocation _box))
  (bind (_x _y _z) (Math|Vector|BreakVector _returnvalue))
  (bind _returnvalue_2 (Math|Vector|MakeVector _x _y _z))
  (bind _returnvalue_3 (Math|Conversions|ToTransform(Vector) _returnvalue_2))
  (if (> (Variables|Default|GetCooldownTimer) 0)
    (Utilities|FlowControl|Delay 1.0)
    (Math|Integer|DecrementInt (Variables|Default|GetCooldownTimer))
    (else
      (Game|SpawnActorfromClass "/Game/TopDownBP/alexsm-test/creeps/melee-creep/BP_MeleeCreep.BP_MeleeCreep_C" _returnvalue_3 "Undefined" 0 0)
      (Game|SpawnActorfromClass "/Game/TopDownBP/alexsm-test/creeps/distance-creep/BP_DistanceCreep.BP_DistanceCreep_C" _returnvalue_3 "Undefined" 0 0)
      (Variables|Default|SetCooldownTimer (Variables|Default|GetCooldownMaxValue))
      (Development|PrintString "Spawned dodics"))))

(event Collision|EventActorBeginOverlap
  (params (OtherActor :type Actor%20Object%20Reference)))

(fn ConstructionScript)